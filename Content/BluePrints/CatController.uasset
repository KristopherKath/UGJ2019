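; CatController turns a left-mouse click-and-drag into a force on the player character.
; On press it stores the deprojected cursor world position, and Tick updates a second position while the button is held.
; Release saves the distance between the two points as a magnitude.
; Whenever the button is up, Tick applies that magnitude, scaled up, equally on all three axes through CharacterMovement AddForce, ignoring drag direction.
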(event `self.ReceiveTick`
  (params (DeltaSeconds :type "Float (single-precision)"))
  (bind _returnvalue (`GameplayStatics.GetPlayerController` 0))
  (bind _returnvalue_2 (* (`self.Magnitude`) 1000.0))
  (bind _returnvalue_3 (`WidgetLayoutLibrary.GetMousePositionOnViewport`))
  (if (`self.IsInputKeyDown` _returnvalue "LeftMouseButton")
    (bind _output_get (set `self.HoldingClick` (`GameplayStatics.DeprojectScreenToWorld` _returnvalue _returnvalue_3)))
    (else
      (`CharacterMovementComponent.AddForce` (`Character.CharacterMovement` (`self.playerCharacter`)) (`KismetMathLibrary.MakeVector` _returnvalue_2 _returnvalue_2 _returnvalue_2)))))

(event `Key|LeftMouseButton`
  (params (Key :type "Key Structure"))
  (:`Pressed`
    (bind _output_get (set `self.FirstClicked` (`self.DeprojectMousePositionToWorld` (`GameplayStatics.GetPlayerController` 0)))))
  (:`Released`
    (set `self.Magnitude` (`KismetMathLibrary.Vector_Distance` _output_get (stale `self.ReceiveTick` _output_get)))))

(event `self.ReceiveBeginPlay`
  (set `self.playerCharacter` (`GameplayStatics.GetPlayerCharacter` 0)))

(fn `UserConstructionScript`)